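; Interactable quest-system actor that shows a text prompt when the player slime (PhysicsSlimeBP1) comes within range.
; Overlapping the Vision sphere, sized by SizeOfVision at construction, reveals the text and plays a timeline that yaws the whole actor toward the slime; leaving hides and stops it.
; OrganizeInEditor snaps the actor to its attach parent.
; AI perception is abandoned for colliders, leaving a debug print and unreachable look-at logic.
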(event OnTargetPerceptionUpdated(AIPerception)
  (params (Actor :type Actor%20Object%20Reference) (Stimulus :type AI%20Stimulus%20Structure))
  ;[1 1 1] Don't Use Perception Used Colliders Instead
  (Development|PrintString "Hello"))

(event OnComponentBeginOverlap(Vision)
  (params (OverlappedComponent :type Primitive%20Component%20Object%20Reference) (OtherActor :type Actor%20Object%20Reference) (OtherComp :type Primitive%20Component%20Object%20Reference) (OtherBodyIndex :type Integer) (bFromSweep :type Boolean) (SweepResult :type Hit%20Result%20Structure%20%28by%20ref%29))
  (bind _asphysics_slime_bp1 (Utilities|Casting|CastToPhysicsSlimeBP1 OtherActor))
  (Rendering|SetVisibility (Variables|Default|GetTextRender) true false)
  (Timeline|VisionLookAt Play
    (:Update
      (CallFunction|RotateTextTowardPlayer (Transformation|GetActorLocation _asphysics_slime_bp1)))))

(event OnComponentEndOverlap(Vision)
  (params (OverlappedComponent :type Primitive%20Component%20Object%20Reference) (OtherActor :type Actor%20Object%20Reference) (OtherComp :type Primitive%20Component%20Object%20Reference) (OtherBodyIndex :type Integer))
  (Utilities|Casting|CastToPhysicsSlimeBP1 OtherActor)
  (Rendering|SetVisibility (Variables|Default|GetTextRender) false false)
  (Timeline|VisionLookAt Stop
    (:Update
      (CallFunction|RotateTextTowardPlayer (Transformation|GetActorLocation (stale OnComponentBeginOverlap(Vision) _asphysics_slime_bp1))))))

(fn ConstructionScript
  (Components|Sphere|SetSphereRadius (Variables|Default|GetVision) (Variables|Default|GetSizeOfVision) true))

(fn OrganizeinEditor
  (Transformation|SetActorLocation (Transformation|GetActorLocation (Actor|GetAttachParentActor)) false false))

(fn RotateTextTowardPlayer
  (params (LookAtVector :type Vector))
  (Transformation|SetActorRotation (Math|Rotator|MakeRotator 0.0 0.0 (.Yaw (Math|Rotator|BreakRotator (Math|Rotator|FindLookatRotation (Transformation|GetWorldLocation (Variables|Default|GetVision)) LookAtVector))))))
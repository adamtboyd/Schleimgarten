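; Safepoint Blueprint that provides a lookup for the safepoint closest to a given location, noted as the Slime's.
; FindNearestSafepoint linearly scans the supplied actor array, comparing each actor's distance to the reference location and returning the closest.
; The search starts from a fixed 9999-unit limit, so it falls back to the first element when none is nearer.
; The event graph and construction script hold no logic.
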(event EventBeginPlay)

(event Collision|EventActorBeginOverlap
  (params (OtherActor :type Actor%20Object%20Reference)))

(event EventTick
  (params (DeltaSeconds :type Float%20%28single-precision%29)))

(fn ConstructionScript)

(fn FindNearestSafepoint
  (params (ActorArray :type Array%20of%20Actor%20Object%20References) (ReferenceLocation :type Vector))
  (LocalVariables|SetNearestDistance 9999.0) ; Reinitialize distance to large value
  (LocalVariables|SetLoc_NearestActor (Utilities|Array|Get(acopy) (Variables|Default|GetActorArray))) ; Set first Safepoint as nearest
  (for _array_element ActorArray
    (if (< (Math|Vector|Distance(Vector) (Transformation|GetActorLocation _array_element) ReferenceLocation) (LocalVariables|GetNearestDistance))
      (LocalVariables|SetNearestDistance (Math|Vector|Distance(Vector) (Transformation|GetActorLocation _array_element) ReferenceLocation))
      (LocalVariables|SetLoc_NearestActor _array_element)))
  (return (LocalVariables|GetLoc_NearestActor)) ; Returns closest actor to Slime
)
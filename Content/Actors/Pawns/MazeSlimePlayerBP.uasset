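; Player pawn for a maze game that steers two slime physics balls at once, the split one with mirrored Y input.
; Movement axes apply velocity-change impulses to both balls, gated by a shared movement state.
; Each tick zeroes their velocity when stationary or interacting, otherwise caps horizontal speed using the actor's velocity.
; An overhead camera follows the balls' midpoint, rising as they separate; look inputs do nothing.
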(event EventBeginPlay
  (|CallParentFunction))

(event EventTick
  (params (DeltaSeconds :type Float%20%28single-precision%29))
  (CallFunction|VelocityLimiter (Variables|Default|GetsplitSlimeBall))
  (CallFunction|VelocityLimiter (Variables|Default|GetslimeBall))
  (CallFunction|PositionOverheadCamera))

(event Input|AxisEvents|InputAxisMoveRight
  (params (AxisValue :type Float%20%28single-precision%29))
  (CallFunction|ImpulseMove (stale Input|AxisEvents|InputAxisMoveForward AxisValue) AxisValue (Variables|Default|GetslimeBall))
  (CallFunction|ImpulseMoveInvertY (stale Input|AxisEvents|InputAxisMoveForward AxisValue) AxisValue (Variables|Default|GetsplitSlimeBall)))

(event Input|AxisEvents|InputAxisMoveForward
  (params (AxisValue :type Float%20%28single-precision%29))
  (CallFunction|ImpulseMove AxisValue (stale Input|AxisEvents|InputAxisMoveRight AxisValue) (Variables|Default|GetslimeBall))
  (CallFunction|ImpulseMoveInvertY AxisValue (stale Input|AxisEvents|InputAxisMoveRight AxisValue) (Variables|Default|GetsplitSlimeBall)))

(event Input|AxisEvents|InputAxisLookUp
  (params (AxisValue :type Float%20%28single-precision%29))
  (CallFunction|DoNothing))

(event Input|AxisEvents|InputAxisTurn
  (params (AxisValue :type Float%20%28single-precision%29))
  (CallFunction|DoNothing))

(fn ConstructionScript
  (|CallParentFunction))

(fn GetPositionDelta
  (params (Pos :type Transform) (Pos' :type Transform)))

(fn ImpulseMove
  (params (ForwardAxisValue :type Float%20%28single-precision%29) (RightAxisValue :type Float%20%28single-precision%29) (TargetBody :type Primitive%20Component%20Object%20Reference))
  (switch Utilities|FlowControl|Switch|SwitchonPlayerState (Variables|Default|GetCurrentState)
    (:NewEnumerator0
      (if (not (and (== ForwardAxisValue 0.0) (== RightAxisValue 0.0)))
        (CallFunction|ChangeCurrentState 1)
        (Physics|AddImpulse TargetBody (Math|Vector|MakeVector (* (Variables|Default|GetMoveImpulseStrength) ForwardAxisValue) (* (Variables|Default|GetMoveImpulseStrength) RightAxisValue) 0.0) "Root" true :!label _label)
        (switch Utilities|FlowControl|Switch|SwitchonPlayerState (Variables|Default|GetCurrentState)
          (:NewEnumerator1
            (if (and (== ForwardAxisValue 0.0) (== RightAxisValue 0.0))
              (CallFunction|ChangeCurrentState))))))
    (:NewEnumerator1
      (goto _label))
    (:NewEnumerator2
      (goto _label))))

(fn ImpulseMoveInvertY
  (params (ForwardAxisValue :type Float%20%28single-precision%29) (RightAxisValue :type Float%20%28single-precision%29) (TargetBody :type Primitive%20Component%20Object%20Reference))
  (switch Utilities|FlowControl|Switch|SwitchonPlayerState (Variables|Default|GetCurrentState)
    (:NewEnumerator0
      (if (not (and (== ForwardAxisValue 0.0) (== RightAxisValue 0.0)))
        (CallFunction|ChangeCurrentState 1)
        (Physics|AddImpulse TargetBody (Math|Vector|MakeVector (* ForwardAxisValue (Variables|Default|GetMoveImpulseStrength)) (* (* RightAxisValue (Variables|Default|GetMoveImpulseStrength)) -1.0) 0.0) "Root" true :!label _label)
        (switch Utilities|FlowControl|Switch|SwitchonPlayerState (Variables|Default|GetCurrentState)
          (:NewEnumerator1
            (if (and (== ForwardAxisValue 0.0) (== RightAxisValue 0.0))
              (CallFunction|ChangeCurrentState))))))
    (:NewEnumerator1
      (goto _label))
    (:NewEnumerator2
      (goto _label))))

(fn VelocityLimiter
  (params (TargetBody :type Primitive%20Component%20Object%20Reference))
  (bind _returnvalue (Transformation|GetVelocity))
  (bind _maxvelocity (Variables|Default|GetMaxVelocity))
  (bind (_x _y _z) (Math|Vector|BreakVector _returnvalue))
  (bind _returnvalue_2 (Math|Vector|MakeVector _x _y 0.0))
  (bind _returnvalue_3 (Math|Vector|ClampVectorSize _returnvalue_2 0.0 _maxvelocity))
  (bind (_x_2 _y_2) (Math|Vector|BreakVector _returnvalue_3))
  (switch Utilities|FlowControl|Switch|SwitchonPlayerState (Variables|Default|GetCurrentState)
    (:NewEnumerator0
      (Physics|SetPhysicsLinearVelocity TargetBody "0, 0, 0" false "None" :!label _label))
    (:NewEnumerator3
      (goto _label))
    (:NewEnumerator1
      (if (> (Math|Vector|VectorLength _returnvalue_2) (Variables|Default|GetMaxVelocity)) :!label _label_2
        (Physics|SetPhysicsLinearVelocity TargetBody (Math|Vector|MakeVector _x_2 _y_2 _z) false "None")))
    (:NewEnumerator2
      (goto _label_2))))

(fn DoNothing)

(fn PositionOverheadCamera
  (bind _slimeball (Variables|Default|GetslimeBall))
  (bind _splitslimeball (Variables|Default|GetsplitSlimeBall))
  (bind _returnvalue (Transformation|GetWorldLocation _slimeball))
  (bind _returnvalue_2 (Transformation|GetWorldLocation _splitslimeball))
  (bind (_x _y _z) (Math|Vector|BreakVector _returnvalue))
  (bind (_x_2 _y_2 _z_2) (Math|Vector|BreakVector _returnvalue_2))
  (Transformation|SetWorldLocation (Variables|Default|GetCamera) (Math|Vector|MakeVector (/ (+ _x_2 _x) 2.0) (/ (+ _y _y_2) 2.0) (+ (/ (+ _z _z_2) 2.0) (/ (Math|Vector|Distance2D(Vector) _returnvalue _returnvalue_2) (Variables|Default|GetCamHeightRatio)))) false false))